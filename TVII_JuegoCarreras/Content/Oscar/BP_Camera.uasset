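; A placed camera actor that becomes the player's view when BP_Tridimina enters its trigger box, for zone-based camera switching.
; Overlap sets the pawn's CurrentCam to this camera and switches the player controller's view target to it.
; On BeginPlay, after a zero-second delay, it also activates if the pawn already overlaps the box.
; The construction script applies the exposed trigger transform and extent to the box.
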(event OnComponentBeginOverlap(PlayerTriggerBox)
  (params (OverlappedComponent :type Primitive%20Component%20Object%20Reference) (OtherActor :type Actor%20Object%20Reference) (OtherComp :type Primitive%20Component%20Object%20Reference) (OtherBodyIndex :type Integer) (bFromSweep :type Boolean) (SweepResult :type Hit%20Result%20Structure%20%28by%20ref%29))
  (bind _asbp_tridimina (Utilities|Casting|CastToBP_Tridimina OtherActor))
  (Variables|/Game/ArturoEscobar/Blueprints/Tridimina/BP_Tridimina.BP_Tridimina_C|SetcurrentCam _asbp_tridimina self)
  (Game|Player|SetViewTargetwithBlend (Game|GetPlayerController 0) self 0.0 "VTBlend_Linear" 0.0 false))

(event EventBeginPlay
  (Utilities|FlowControl|Delay 0.0)
  (bind _asbp_tridimina (Utilities|Casting|CastToBP_Tridimina (Game|Player|GetPlayerPawn 0)))
  (for _array_element (Class|Actor|GetOverlappingComponents _asbp_tridimina)
    (if (== _array_element (Variables|Default|GetPlayerTriggerBox))
      (Variables|/Game/ArturoEscobar/Blueprints/Tridimina/BP_Tridimina.BP_Tridimina_C|SetcurrentCam _asbp_tridimina self)
      (Game|Player|SetViewTargetwithBlend (Game|GetPlayerController 0) self 0.0 "VTBlend_Linear" 0.0 false))))

(fn ConstructionScript
  (Transformation|SetRelativeTransform (Variables|Default|GetPlayerTriggerBox) (Variables|Default|GetPlayer%20Trigger%20Transform) false false)
  (Components|Box|SetBoxExtent (Variables|Default|GetPlayerTriggerBox) (Variables|Default|GetPlayer%20Trigger%20Extend) true))